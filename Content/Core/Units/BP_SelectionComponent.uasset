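; Actor component that marks its owning unit as selected with a ground decal indicator.
; On BeginPlay it adds a rotated decal component to the owner, applies the selection indicator material, hides it, then scales it to IndicatorRadius and moves it to IndicatorOffset.
; ShowSelectiondecal and HideSelectionDecal toggle the decal's visibility and hidden-in-game state.
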(event `self.ReceiveBeginPlay`
  (bind _indicatorradius (`self.IndicatorRadius`))
  (bind (_decalsize_x _decalsize_y _decalsize_z) (`KismetMathLibrary.BreakVector` (`DecalComponent.DecalSize` (`self.DecalComponentReference`))))
  (bind _returnvalue (`|AddComponentByClass` (`self.GetOwner`) "/Script/Engine.DecalComponent" false (`KismetMathLibrary.MakeTransform` (0.0 0.0 0.0) (struct :`Pitch` 90.0))))
  (set `self.DecalComponentReference` _returnvalue)
  (`DecalComponent.SetDecalMaterial` (`self.DecalComponentReference`) "/Game/Core/Building/MI_SelectionIndicator.MI_SelectionIndicator")
  (`self.HideSelectionDecal`)
  (`SceneComponent.SetRelativeScale3D` (`self.DecalComponentReference`) (`KismetMathLibrary.MakeVector` 128.0 (/ _indicatorradius _decalsize_y) (/ _indicatorradius _decalsize_z)))
  (`SceneComponent.K2_SetRelativeLocation` (`self.DecalComponentReference`) (`self.IndicatorOffset`) false false))

(event `ShowSelection decal`
  (bind _decalcomponentreference (`self.DecalComponentReference`))
  ;[1 1 1] Show Selected unit
  (`SceneComponent.SetVisibility` _decalcomponentreference true false)
  (`SceneComponent.SetHiddenInGame` _decalcomponentreference false false))

(event `HideSelectionDecal`
  (bind _decalcomponentreference (`self.DecalComponentReference`))
  ;[1 1 1] Hide Selected unit
  (`SceneComponent.SetVisibility` _decalcomponentreference false false)
  (`SceneComponent.SetHiddenInGame` _decalcomponentreference true false))