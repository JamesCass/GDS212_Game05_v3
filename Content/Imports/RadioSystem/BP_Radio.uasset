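; BP_Radio is a radio Blueprint meant to play random songs from SongList as 2D sound.
; SelectNewSong re-rolls until the pick differs from the current song, and FadeOut fades out any valid playing audio component.
; A chain fades out, picks, spawns the sound, waits its duration and calls ChangeSong to repeat.
; That chain is disconnected and BeginPlay and ChangeSong are empty, so nothing plays as wired.
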(event `self.ReceiveBeginPlay`)

(event `Change Song`)

(fn `FadeOut`
  (returns (`Faded out?` :type Boolean))
  (bind _current_song_ref (`self.Current song ref`)
    (:`then`
      (`AudioComponent.FadeOut` _current_song_ref (`self.Fade Duration`) 0.0 "Linear")
      (return true))
    (:`else`
      (return false))))

(fn `Select new song`
  (returns (`Selected Song` :type "SoundBase Object Reference"))
  (locals (`Provi Song` :type "SoundBase Object Reference"))
  (bind _song_list (`self.Song list`))
  (set `local.Provi Song` (`|GetArrayItem` _song_list (`KismetMathLibrary.RandomIntegerInRange` 0 (`KismetArrayLibrary.Array_LastIndex` _song_list))) :!label _label)
  (if (== (`self.Current Song sound base`) (`local.Provi Song`))
    (goto _label)
    (else
      (return (`local.Provi Song`)))))

(fn `UserConstructionScript`)