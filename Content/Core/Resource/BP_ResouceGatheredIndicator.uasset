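; BP_ResouceGatheredIndicator is a short-lived visual indicator actor for gathered resources, showing a configurable mesh that moves upward.
; The construction script assigns MeshToUse to ResourceMesh.
; On BeginPlay, a sped-up timeline drives the mesh's relative Z from an alpha scaled by MaxUpwardDistance, then destroys the actor when finished.
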(event `self.ReceiveBeginPlay`
  (`TimelineComponent.SetPlayRate` (`self.UpwardsAnimation`) 1.7)
  (bind (_direction _zvaluealpha) (`Timeline|UpwardsAnimation`)
    (:`Update`
      (`SceneComponent.K2_SetRelativeLocation` (`self.ResourceMesh`) (`KismetMathLibrary.MakeVector` 0.0 0.0 (* _zvaluealpha (`self.MaxUpwardDistance`))) false false))
    (:`Finished`
      (`self.K2_DestroyActor`))))

(fn `UserConstructionScript`
  (`StaticMeshComponent.SetStaticMesh` (`self.ResourceMesh`) (`self.MeshToUse`)))