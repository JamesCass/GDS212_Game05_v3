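; RTS worker unit that takes move, attack, gather and building-interaction orders, and can be click-selected when friendly.
; AIMoveTo drives each order, while BPUnitComponent state changes select looping knight or skeleton animations by alliance.
; Attacks apply damage on a looping timer, chasing targets that leave range.
; Gathering waits out a retriggerable delay, deposits at the town hall through the player controller, then repeats while the resource remains mineable.
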(event `/Game/Core/Units/BPI_UnitActions.AttackThisActor`
  (params (ActorToAttack :type "Actor Object Reference"))
  (bind _actor_to_attack (`self.Actor to Attack`))
  (bind _returnvalue (`self.GetComponentByClass` (`self.Actor to Attack`) "/Game/Core/Building/BP_BuildingComponent.BP_BuildingComponent_C"))
  (bind (_returnvalue_roll _returnvalue_pitch _returnvalue_yaw) (`KismetMathLibrary.BreakRotator` (`KismetMathLibrary.FindLookAtRotation` (`self.K2_GetActorLocation`) (`self.K2_GetActorLocation` (`self.Actor to Attack`)))))
  ;[0 0 0] Attack Order
  (set `self.Actor to Attack` ActorToAttack)
  (`/Game/Core/Units/BP_UnitComponent.HandleNewUnitState` (`self.BP_UnitComponent`) "NewEnumerator2")
  (`/Engine/EditorBlueprintResources/StandardMacros.IsValid` _returnvalue
    (:`Is Valid`
      (`|AIMoveTo` self (`SceneComponent.K2_GetComponentLocation` (`/Game/Core/Building/BP_BuildingComponent.Get Suitable Location` _returnvalue)) null 200.0 true
        (:`OnSuccess`
          _)))
    (:`Is Not Valid`
      (`|AIMoveTo` self (0.0 0.0 0.0) (`self.Actor to Attack`) 200.0 true
        (:`OnSuccess`
          _))))
  (`/Engine/EditorBlueprintResources/StandardMacros.IsValid` _actor_to_attack
    (:`Is Valid`
      (set `self.RangeToActorToAttack` (`KismetMathLibrary.Vector_Distance` (`self.K2_GetActorLocation` _actor_to_attack) (`self.K2_GetActorLocation`)))
      (`self.K2_SetActorRotation` (`KismetMathLibrary.MakeRotator` 0.0 0.0 _returnvalue_yaw))
      (`/Game/Core/Units/BP_UnitComponent.HandleNewUnitState` (`self.BP_UnitComponent`) "NewEnumerator4")
      (bind _returnvalue_2 (`KismetSystemLibrary.K2_SetTimerDelegate` (`|CreateDelegate` :!event `AttackFunction`) 1.0 true))
      (set `self.AttackEventTimer` _returnvalue_2))
    (:`Is Not Valid`
      (`self.StopAttack`))))

(event `self.ReceiveBeginPlay`)

(event `AttackFunction`
  (bind _actor_to_attack (`self.Actor to Attack`))
  ;[0 0 0] Attack Order
  (`self.Actor to Attack`
    (:`then`
      (if (<= (`KismetMathLibrary.Vector_Distance` (`self.K2_GetActorLocation` (`self.Actor to Attack`)) (`self.K2_GetActorLocation`)) (`self.RangeToActorToAttack`))
        (`GameplayStatics.ApplyDamage` (`self.Actor to Attack`) (`/Game/Core/Units/BP_UnitComponent.Damage` (`self.BP_UnitComponent`)))
        (else
          (`KismetSystemLibrary.K2_ClearAndInvalidateTimerHandle` (`self.AttackEventTimer`))
          (if (`|EnumEquality` (`/Game/Core/Units/BP_UnitComponent.UnitState` (`self.BP_UnitComponent`)) "NewEnumerator4")
            (`/Engine/EditorBlueprintResources/StandardMacros.IsValid` _actor_to_attack
              (:`Is Valid`
                (`/Game/Core/Units/BPI_UnitActions.AttackThisActor` _actor_to_attack)))))))
    (:`else`
      (`self.StopAttack`))))

(event `StopAttack`
  ;[0 0 0] Attack Order
  (`/Game/Core/Units/BP_UnitComponent.HandleNewUnitState` (`self.BP_UnitComponent`) "NewEnumerator1")
  (`KismetSystemLibrary.K2_ClearAndInvalidateTimerHandle` (`self.AttackEventTimer`)))

(event `/Game/Core/Units/BPI_UnitActions.MoveToThisLocation`
  (params (GoalLocation :type "Vector Structure"))
  ;[0 0 0] Move to location Order
  (`/Game/Core/Units/BP_UnitComponent.HandleNewUnitState` (`self.BP_UnitComponent`) "NewEnumerator2")
  (bind _movementresult (`|AIMoveTo` self GoalLocation null 50.0)
    (:`OnSuccess`
      _)
    (:`OnFail`
      (switch `EPathFollowingResult` _movementresult
        (:`Blocked`
          _)
        (:`OffPath`
          _)
        (:`Invalid`
          _))))
  (`/Game/Core/Units/BP_UnitComponent.HandleNewUnitState` (`self.BP_UnitComponent`) "NewEnumerator1"))

(event `/Game/Core/Units/BPI_UnitActions.GatherThisResource`
  (params (ResourceRef :type "Actor Object Reference"))
  (bind _returnvalue (`self.GetComponentByClass` ResourceRef "/Game/Core/Resource/BP_resourceComponent.BP_resourceComponent_C"))
  (bind (_returnvalue_roll _returnvalue_pitch _returnvalue_yaw) (`KismetMathLibrary.BreakRotator` (`KismetMathLibrary.FindLookAtRotation` (`self.K2_GetActorLocation`) (`self.K2_GetActorLocation` ResourceRef))))
  ;[0 0 0] Gather Resource Order
  ;;[0 0 0] Move to the resource
  (`/Game/Core/Units/BP_UnitComponent.HandleNewUnitState` (`self.BP_UnitComponent`) "NewEnumerator2")
  (`|AIMoveTo` self (0.0 0.0 0.0) ResourceRef 200.0
    (:`OnSuccess`
      (`self.K2_SetActorRotation` (`KismetMathLibrary.MakeRotator` 0.0 0.0 _returnvalue_yaw))
      ;;[0 0 0] Start gathering Resource
      (if (and (`/Game/Core/Resource/BP_resourceComponent.CanThisResourceBeMined` _returnvalue) (`|EnumInequality` (`self.ResourceBeingCarried`) (`/Game/Core/Resource/BP_resourceComponent.TypeofResource` _returnvalue)))
        (`/Game/Core/Units/BP_UnitComponent.HandleNewUnitState` (`self.BP_UnitComponent`) "NewEnumerator3")
        (set `self.AmountOfResource` 0)
        (`KismetSystemLibrary.RetriggerableDelay` (`/Game/Core/Resource/BP_resourceComponent.TimeToBeGatheredInSeconds` _returnvalue))
        ;;[0 0 0] resource collected
        (if (`|EnumEquality` (`/Game/Core/Units/BP_UnitComponent.UnitState` (`self.BP_UnitComponent`)) "NewEnumerator3")
          (bind (_typeofresource _numberresourcestogive) (`/Game/Core/Resource/BP_resourceComponent.GiveResource` _returnvalue))
          (set `self.ResourceBeingCarried` _typeofresource)
          (set `self.AmountOfResource` _numberresourcestogive)
          (`self.GotoTownHallAndDeposit` ResourceRef))
        (elif (and (`|EnumEquality` (`self.ResourceBeingCarried`) (`/Game/Core/Resource/BP_resourceComponent.TypeofResource` _returnvalue)) (> (`self.AmountOfResource`) 0))
          (`self.GotoTownHallAndDeposit` ResourceRef)
          (else
            (`/Game/Core/Units/BP_UnitComponent.HandleNewUnitState` (`self.BP_UnitComponent`) "NewEnumerator1")))))))

(event `GotoTownHallAndDeposit`
  (params (`resource ref` :type "Actor Object Reference"))
  (`/Game/Core/Units/BP_UnitComponent.HandleNewUnitState` (`self.BP_UnitComponent`) "NewEnumerator2")
  (bind _asbp_rts_game_mode (cast `/Game/Core/Framework/BP_RTS_GameMode` (`GameplayStatics.GetGameMode`)))
  (bind _suitablelocationref (`/Game/Core/Building/BP_BuildingComponent.Get Suitable Location` (`self.GetComponentByClass` (`/Game/Core/Framework/BP_RTS_GameMode.GetPlayerTownHall` _asbp_rts_game_mode) "/Game/Core/Building/BP_BuildingComponent.BP_BuildingComponent_C")))
  (`/Engine/EditorBlueprintResources/StandardMacros.IsValid` _suitablelocationref
    (:`Is Valid`
      (`|AIMoveTo` self (`SceneComponent.K2_GetComponentLocation` _suitablelocationref) null 200.0 true
        (:`OnSuccess`
          (`/Game/Core/Units/BP_UnitComponent.HandleNewUnitState` (`self.BP_UnitComponent`) "NewEnumerator2")
          (bind _asbp_player_controller (cast `/Game/Core/Player/BP_PlayerController` (`GameplayStatics.GetPlayerController` 0)))
          (`/Game/Core/Player/BP_PlayerController.RecieveRecourse` _asbp_player_controller (`self.ResourceBeingCarried`) (`self.AmountOfResource`))
          (set `self.ResourceBeingCarried` "NewEnumerator0")
          (set `self.AmountOfResource` 0)
          (`/Engine/EditorBlueprintResources/StandardMacros.IsValid` `resource ref`
            (:`Is Valid`
              (`self.RepeatTheMiningAction` `resource ref`))))))
    (:`Is Not Valid`
      (`/Game/Core/Units/BP_UnitComponent.HandleNewUnitState` (`self.BP_UnitComponent`) "NewEnumerator1"))))

(event `RepeatTheMiningAction`
  (params (ResourceRef :type "Actor Object Reference"))
  ;[0 0 0] Repeat the mining action if stopped
  (if (`/Game/Core/Resource/BP_resourceComponent.CanThisResourceBeMined` (`self.GetComponentByClass` ResourceRef "/Game/Core/Resource/BP_resourceComponent.BP_resourceComponent_C"))
    (`/Game/Core/Units/BPI_UnitActions.GatherThisResource` ResourceRef)))

(event `self.BP_UnitComponent.OnEnterNewState`
  (params (NewState :type "/Game/Core/Units/E_UnitStates Enum" :default "NewEnumerator0"))
  ;[0 0 0] State and animation handler
  (if (`|EnumEquality` (`/Game/Core/Units/BP_UnitComponent.Alliance` (`self.BP_UnitComponent`)) "Friendly")
    (`SkeletalMeshComponent.PlayAnimation` (`self.Mesh`) (select `/Game/Core/Units/E_UnitStates` NewState :`NewEnumerator1` "/Game/Imports/Humans/Knight_Anim_Idle.Knight_Anim_Idle" :`NewEnumerator2` "/Game/Imports/Humans/Knight_Anim_Walking_B.Knight_Anim_Walking_B" :`NewEnumerator3` "/Game/Imports/Humans/Knight_Anim_1H_Melee_Attack_Chop.Knight_Anim_1H_Melee_Attack_Chop" :`NewEnumerator4` "/Game/Imports/Humans/Knight_Anim_1H_Melee_Attack_Slice_Diagonal.Knight_Anim_1H_Melee_Attack_Slice_Diagonal" :!type "AnimationAsset Object Reference") true)
    (elif (`|EnumEquality` (`/Game/Core/Units/BP_UnitComponent.Alliance` (`self.BP_UnitComponent`)) "Hostile")
      (`SkeletalMeshComponent.PlayAnimation` (`self.Mesh`) (select `/Game/Core/Units/E_UnitStates` NewState :`NewEnumerator1` "/Game/Imports/Enemies/Skeleton_Minion_Anim_Idle.Skeleton_Minion_Anim_Idle" :`NewEnumerator2` "/Game/Imports/Enemies/Skeleton_Minion_Anim_Walking_C.Skeleton_Minion_Anim_Walking_C" :`NewEnumerator3` "/Game/Imports/Humans/Knight_Anim_1H_Melee_Attack_Chop.Knight_Anim_1H_Melee_Attack_Chop" :`NewEnumerator4` "/Game/Imports/Enemies/Skeleton_Minion_Anim_1H_Melee_Attack_Stab.Skeleton_Minion_Anim_1H_Melee_Attack_Stab" :!type "AnimationAsset Object Reference") true))))

(event `/Game/Core/Units/BPI_UnitActions.InteractWithBuilding`
  (params (BuildingRef :type "Actor Object Reference"))
  (bind _returnvalue (`self.GetComponentByClass` BuildingRef "/Game/Core/Building/BP_BuildingComponent.BP_BuildingComponent_C"))
  (`/Engine/EditorBlueprintResources/StandardMacros.IsValid` _returnvalue
    (:`Is Valid`
      (if (> (`self.AmountOfResource`) 0)
        (if (`|EnumEquality` (`/Game/Core/Building/BP_BuildingComponent.TypeOfBuilding` _returnvalue) "NewEnumerator1")
          (`self.GotoTownHallAndDeposit` null))))))

(event `/Game/Core/Building/BPI_SelectionEvents.SelectThis`
  (`/Game/Core/Units/BP_SelectionComponent.ShowSelection decal` (`self.BP_SelectionComponent`)))

(event `/Game/Core/Building/BPI_SelectionEvents.DeselectThis`
  (`/Game/Core/Units/BP_SelectionComponent.HideSelectionDecal` (`self.BP_SelectionComponent`)))

(event `self.CapsuleComponent.OnClicked`
  (params (TouchedComponent :type "PrimitiveComponent Object Reference") (ButtonPressed :type "Key Structure"))
  (if (`|EnumEquality` (`/Game/Core/Units/BP_UnitComponent.Alliance` (`self.BP_UnitComponent`)) "Friendly")
    (message `/Game/Core/Building/BPI_SelectionEvents.ClickSelectThisActor` (`GameplayStatics.GetPlayerController` 0) self)))

(fn `GetTeamAttitude`
  (returns (TeamAttitude :type "ETeamAttitude Enum"))
  (return (`/Game/Core/Units/BP_UnitComponent.Alliance` (`self.BP_UnitComponent`))))

(fn `UserConstructionScript`)