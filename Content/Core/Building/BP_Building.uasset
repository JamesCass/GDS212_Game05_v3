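; BP_Building is a building actor that the player can select with a click.
; A click calls BuildingClicked, which registers the actor in BP_PlayerController's selected-actor list and shows its SelectionDecal.
; DeselectThis hides the decal again without changing that list.
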(event `self.ReceiveActorOnClicked`
  (params (ButtonPressed :type "Key Structure"))
  (`self.BuildingClicked`))

(event `BuildingClicked`
  (bind _selectiondecal (`self.SelectionDecal`))
  (`|ExecutionSequence`
    (:`then_0`
      (bind _asbp_player_controller (cast `/Game/Core/Player/BP_PlayerController` (`GameplayStatics.GetPlayerController` 0)))
      (`/Game/Core/Player/BP_PlayerController.AddActorSelectedToList` _asbp_player_controller self))
    (:`then_1`
      (`SceneComponent.SetHiddenInGame` _selectiondecal false false)
      (`SceneComponent.SetVisibility` _selectiondecal true false))))

(event `/Game/Core/Building/BPI_SelectionEvents.DeselectThis`
  (bind _selectiondecal (`self.SelectionDecal`))
  (`SceneComponent.SetHiddenInGame` _selectiondecal true false)
  (`SceneComponent.SetVisibility` _selectiondecal false false))

(fn `UserConstructionScript`)