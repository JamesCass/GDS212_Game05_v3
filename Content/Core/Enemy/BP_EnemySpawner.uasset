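; BP_EnemySpawner is an actor that periodically spawns waves of BP_Worker_Tribe2 enemies around itself.
; On BeginPlay it starts a looping timer at the WaveTimer interval, and each tick requests a small random number of spawns.
; Each enemy appears at a random navigable point within the SphereCol radius, raised slightly and always spawned regardless of collision.
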(event `self.ReceiveBeginPlay`
  (bind _returnvalue (`KismetSystemLibrary.K2_SetTimerDelegate` (delegate `AddSpawnWave`) (`self.WaveTimer`) true 0.0 2.0))
  (set `self.SpawnTimer` _returnvalue))

(event `AddSpawnWave`
  (`self.SpawnEnemy` (`KismetMathLibrary.RandomIntegerInRange` 1 2)))

(event `SpawnEnemy`
  (params (EnemiesToSpawn :type Integer :default 1))
  (for _ (range 1 (+ EnemiesToSpawn 1))
    (bind _randomlocation (`NavigationSystemV1.K2_GetRandomLocationInNavigableRadius` (`self.K2_GetActorLocation`) (`SphereComponent.GetScaledSphereRadius` (`self.SphereCol`)) null null))
    (`|SpawnActorFromClass` "/Game/Units/Tribe2/BP_Worker_Tribe2.BP_Worker_Tribe2_C" (`KismetMathLibrary.MakeTransform` (+ _randomlocation (0.0 0.0 100.0))) "AlwaysSpawn" "MultiplyWithRoot" null null)))

(fn `UserConstructionScript`)