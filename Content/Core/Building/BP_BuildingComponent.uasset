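; BP_BuildingComponent gives its owning building health, a health bar and go-to locations.
; On BeginPlay it adds a BP_HealthComponent bar to the owner and binds to its damage event.
; Damage lowers Health, refreshes the bar and broadcasts OnDestroy with the Alliance at zero.
; GetSuitableLocation flags a random BP_GoLocation as full and returns a separately re-rolled pick, without checking IsFull.
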(event `self.ReceiveBeginPlay`
  (bind _returnvalue (`self.GetOwner`))
  (`|ExecutionSequence`
    (:`then_0`
      (bind _returnvalue_2 (`|AddComponentByClass` _returnvalue "/Game/Core/Units/BP_HealthComponent.BP_HealthComponent_C" false (`KismetMathLibrary.MakeTransform` (`self.HealthBarLocation`))))
      (`WidgetComponent.SetDrawSize` _returnvalue_2 (`self.HealthBarSize`))
      (`self.UpdateHealthBar`))
    (:`then_1`
      (add `Actor.OnTakeAnyDamage` _returnvalue (`|CreateDelegate` :!event `OnOwnerTakeAnyDamage`)))))

(event `OnOwnerTakeAnyDamage`
  (params (DamagedActor :type "Actor Object Reference") (Damage :type "Float (single-precision)") (DamageType :type "DamageType Object Reference") (InstigatedBy :type "Controller Object Reference") (DamageCauser :type "Actor Object Reference"))
  (set `self.Health` (`KismetMathLibrary.FMax` (- (`self.Health`) Damage)))
  (`self.UpdateHealthBar`)
  (if (<= (`self.Health`) 0.0)
    (`self.OnDestroy` (`self.Alliance`))))

(fn `Get Suitable Location`
  (returns (SuitableLocationRef :type "/Game/Core/Building/BP_GoLocation Object Reference"))
  (bind _returnvalue (`Actor.K2_GetComponentsByClass` (`self.GetOwner`) "/Game/Core/Building/BP_GoLocation.BP_GoLocation_C"))
  (bind _outitem (`KismetArrayLibrary.Array_Random` _returnvalue))
  (if (`KismetArrayLibrary.Array_IsNotEmpty` _returnvalue)
    (set `/Game/Core/Building/BP_GoLocation.IsFull` true _outitem)
    (return _outitem)
    (else
      (return null))))

(fn `UpdateHealthBar`
  (bind _returnvalue (`Actor.GetComponentByClass` (`self.GetOwner`) "/Game/Core/Units/BP_HealthComponent.BP_HealthComponent_C"))
  (`/Engine/EditorBlueprintResources/StandardMacros.IsValid` _returnvalue
    (:`Is Valid`
      (`/Game/Core/Units/BP_HealthComponent.UpdateHealthBar` _returnvalue (/ (`self.Health`) (`self.HealthMax`))))
    (:`Is Not Valid`
      (`KismetSystemLibrary.PrintString` "Building missing health component"))))