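; Player controller that pans the controlled pawn as a camera and tracks the selected actor.
; Movement follows control yaw, using axis input or falling back to screen-edge scrolling scales computed from the mouse's normalized viewport position.
; Adding a selection first clears the SelectedActors list, notifying previous entries through BPI_SelectionEvents, so only one actor stays selected at a time.
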(event `InputAxis|MoveForward`
  (params (AxisValue :type "Float (single-precision)"))
  (bind (_returnvalue_roll _returnvalue_pitch _returnvalue_yaw) (`KismetMathLibrary.BreakRotator` (`self.GetControlRotation`)))
  ;[0 0 0] Camera movement
  (`Pawn.AddMovementInput` (`self.K2_GetPawn`) (`KismetMathLibrary.GetForwardVector` (`KismetMathLibrary.MakeRotator` 0.0 0.0 _returnvalue_yaw)) (`KismetMathLibrary.SelectFloat` AxisValue (`self.MouseForwardScale`) (!= AxisValue 0.0)) false))

(event `InputAxis|MoveRight`
  (params (AxisValue :type "Float (single-precision)"))
  (bind (_returnvalue_roll _returnvalue_pitch _returnvalue_yaw) (`KismetMathLibrary.BreakRotator` (`self.GetControlRotation`)))
  ;[0 0 0] Camera movement
  (`Pawn.AddMovementInput` (`self.K2_GetPawn`) (`KismetMathLibrary.GetRightVector` (`KismetMathLibrary.MakeRotator` 0.0 0.0 _returnvalue_yaw)) (`KismetMathLibrary.SelectFloat` AxisValue (`self.MouseRightScale`) (!= AxisValue 0.0)) false))

(event `InputAxis|MouseMovement`
  (params (AxisValue :type "Float (single-precision)"))
  (bind (_returnvalue_x _returnvalue_y) (`KismetMathLibrary.BreakVector2D` (`WidgetLayoutLibrary.GetViewportSize`)))
  (bind _returnvalue_x_2 (`KismetMathLibrary.BreakVector2D` (`WidgetLayoutLibrary.GetViewportSize`)))
  (bind _returnvalue (/ (`self.GetMousePosition`) _returnvalue_x_2))
  (bind _returnvalue_2 (/ (`.LocationY` (`self.GetMousePosition`)) _returnvalue_y))
  ;[0 0 0] Camera movement
  (set `self.MouseRightScale` (`KismetMathLibrary.SelectFloat` -1.0 (`KismetMathLibrary.SelectFloat` 1.0 0.0 (> _returnvalue (- 1.0 (`self.ViewportEdgeThreshold`)))) (< _returnvalue (`self.ViewportEdgeThreshold`))))
  (set `self.MouseForwardScale` (`KismetMathLibrary.SelectFloat` 1.0 (`KismetMathLibrary.SelectFloat` -1.0 0.0 (> _returnvalue_2 (- 1.0 (`self.ViewportEdgeThreshold`)))) (< _returnvalue_2 (`self.ViewportEdgeThreshold`)))))

(event `AddActorSelectedToList`
  (params (SelectedActor :type "Actor Object Reference"))
  (`self.DeselectAllActors`)
  (`KismetArrayLibrary.Array_Add` (`self.SelectedActors`) SelectedActor))

(event `InputAction|MouseSelection`
  (params (Key :type "Key Structure")))

(event `DeselectAllActors`
  (for _array_element (`self.SelectedActors`)
    (if (`KismetSystemLibrary.DoesImplementInterface` _array_element "/Game/Core/Building/BPI_SelectionEvents.BPI_SelectionEvents_C")
      (message `/Game/Core/Building/BPI_SelectionEvents.DeselectThis` _array_element)))
  (`KismetArrayLibrary.Array_Clear` (`self.SelectedActors`)))

(fn `UserConstructionScript`)