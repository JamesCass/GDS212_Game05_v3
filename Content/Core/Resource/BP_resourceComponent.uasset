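; Resource component that makes its owner a gatherable resource with a limited number of harvests.
; GiveResource decrements the remaining-use counter, signals that a resource was gathered, and returns the resource type and amount to give.
; It also signals exhaustion once the counter is no longer above zero.
; CanThisResourceBeMined exposes that counter check, which GiveResource does not test before giving.
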(fn `CanThisResourceBeMined`
  (returns (ReturnValue :type Boolean))
  (return (> (`self.TimesItCanBeTimed`) 0)))

(fn `GiveResource`
  (returns (TypeofResource :type "/Game/Core/Resource/E_ResourceType Enum") (NumberResourcesToGive :type Integer))
  (set `self.TimesItCanBeTimed` (- (`self.TimesItCanBeTimed`) 1))
  (`self.OnResourceGathered`)
  (`|ExecutionSequence`
    (:`then_0`
      (if (not (`self.CanThisResourceBeMined`))
        (`self.OnResourceExhausted`)))
    (:`then_1`
      (return (`self.TypeofResource`) (`self.NumberResourcesToGive`)))))