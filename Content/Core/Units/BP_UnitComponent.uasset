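; BP_UnitComponent is an actor component that makes its owning unit click-selectable and tracks its current state.
; On BeginPlay it binds to the owner's OnClicked event; a click adds the owner to BP_PlayerController's selection list and reveals the owner's DecalComponent as a selection marker.
; HandleNewUnitState stores the new state and fires the matching enter dispatcher for Idle, Movement or Mining.
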(event `self.ReceiveBeginPlay`
  (add `Actor.OnClicked` (`self.GetOwner`) (`|CreateDelegate` :!event `OnOwnerClicked`)))

(event `OnOwnerClicked`
  (params (TouchedActor :type "Actor Object Reference") (ButtonPressed :type "Key Structure" :default "None"))
  (`self.AddUnitToSelectionList`)
  (`self.ShowSelection decal`))

(event `AddUnitToSelectionList`
  (bind _asbp_player_controller (cast `/Game/Core/Player/BP_PlayerController` (`GameplayStatics.GetPlayerController` 0)))
  (`/Game/Core/Player/BP_PlayerController.AddActorSelectedToList` _asbp_player_controller (`self.GetOwner`)))

(event `ShowSelection decal`
  (bind _returnvalue (`Actor.GetComponentByClass` (`self.GetOwner`) "/Script/Engine.DecalComponent"))
  ;[1 1 1] Show Selected unit
  (`SceneComponent.SetVisibility` _returnvalue true false)
  (`SceneComponent.SetHiddenInGame` _returnvalue false false))

(fn `HandleNewUnitState`
  (params (UnitState :type "/Game/Core/Units/E_UnitStates Enum" :default "NewEnumerator0"))
  (bind _output_get (set `self.UnitState` UnitState))
  (switch `/Game/Core/Units/E_UnitStates` _output_get
    (:`NewEnumerator1`
      (`self.OnEnterIdle`))
    (:`NewEnumerator2`
      (`self.OnEnterMovement`))
    (:`NewEnumerator3`
      (`self.OnEnterMining`))))