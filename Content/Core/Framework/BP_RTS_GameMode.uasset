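; BP_RTS_GameMode is the RTS game mode that tracks town halls and handles losing the match.
; BeginPlay caches every BP_TownCentre, but binding their building components' destroy events to OnTownHallDestroyed is disconnected.
; That handler calls GameLost for a Friendly alliance, showing the LoseScreen widget.
; GetPlayerTownHall searches actor tags for "None", then indexes TownHall with the tag's index rather than the actor's.
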(event `self.ReceiveBeginPlay`
  (bind _outactors (`GameplayStatics.GetAllActorsOfClass` "/Game/Buildings/BP_TownCentre.BP_TownCentre_C"))
  (bind _output_get (set `self.TownHall` _outactors))
  (for _array_element _output_get
    _))

(event `OnTownHallDestroyed`
  (params (alliance :type "ETeamAttitude Enum" :default "Friendly"))
  (if (`|EnumEquality` alliance "Friendly")
    (`self.GameLost`)))

(event `GameLost`
  (bind _returnvalue (`|CreateWidget` "/Game/Core/Ui/LoseScreen.LoseScreen_C"))
  (`UserWidget.AddToViewport` _returnvalue 0))

(fn `GetPlayerTownHall`
  (returns (PlayerTownHall :type "Actor Object Reference"))
  (locals (FoundIndex :type Integer))
  (for _array_element (`self.TownHall`)
    (bind _returnvalue (`KismetArrayLibrary.Array_Find` (`Actor.Tags` _array_element)))
    (if (>= _returnvalue 0)
      (set `local.FoundIndex` _returnvalue)
      (break)))
  (return (`|GetArrayItem` (`self.TownHall`) (`local.FoundIndex`))))

(fn `UserConstructionScript`)